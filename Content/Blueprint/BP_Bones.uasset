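; BP_Bones is the player character, which faces its horizontal movement direction and returns to the main menu on death.
; BeginPlay creates HUD widgets for collected pants, weapon and dash cooldowns, and a red hurt overlay, which Tick updates from component and cooldown state.
; Dash, gated by cooldown and a DoOnce, hops then launches toward a target, ignoring Pawn collision and counting as invincible until it ends.
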(event EventBeginPlay
  (bind _returnvalue (UserInterface|CreateWidget "/Game/UI/WBP_Pant.WBP_Pant_C" (Game|GetPlayerController 0)))
  (bind _output_get (Variables|Default|SetPantUI _returnvalue))
  (UserInterface|Viewport|AddtoViewport _output_get 0)
  (bind _returnvalue_2 (UserInterface|CreateWidget "/Game/UI/WBP_WeaponCooldown.WBP_WeaponCooldown_C" (Game|GetPlayerController 0)))
  (bind _output_get_2 (Variables|Default|SetWeaponCooldownUI _returnvalue_2))
  (UserInterface|Viewport|AddtoViewport _output_get_2 0)
  (bind _returnvalue_3 (UserInterface|CreateWidget "/Game/UI/WBP_DashCooldown.WBP_DashCooldown_C" (Game|GetPlayerController 0)))
  (bind _output_get_3 (Variables|Default|SetDashCooldownUI _returnvalue_3))
  (UserInterface|Viewport|AddtoViewport _output_get_3 0)
  (bind _returnvalue_4 (UserInterface|CreateWidget "/Game/UI/WBP_Damaged.WBP_Damaged_C" (Game|GetPlayerController 0)))
  (bind _output_get_4 (Variables|Default|SetRedScreenFade _returnvalue_4))
  (UserInterface|Viewport|AddtoViewport _output_get_4 0)
  (Widget|SetVisibility _output_get_4 "Hidden"))

(event EventPlayerDied
  (Game|OpenLevel(byObjectReference) "/Game/Levels/LVL_MainMenu.LVL_MainMenu"))

(event EventTick
  (params (DeltaSeconds :type Float%20%28single-precision%29))
  (bind _returnvalue (Transformation|GetActorLocation))
  (bind _returnvalue_2 (Transformation|GetActorLocation))
  (bind _returnvalue_3 (Transformation|GetVelocity))
  (bind _health (Variables|Default|GetHealth))
  (bind _redscreenfade (Variables|Default|GetRedScreenFade))
  (bind _ishurt (Variables|/Script/SkellHell.Health|GetIsHurt _health))
  (Utilities|FlowControl|Sequence
    (:then_0
      (CallFunction|PantUIUpdate)
      (CallFunction|WeaponCooldownUIUpdate)
      (Variables|Default|SetDashCooldownTime (+ DeltaSeconds (Variables|Default|GetDashCooldownTime)))
      (CallFunction|DashCooldownUIUpdate)
      (if (and _ishurt (not (Variables|Default|GetRedScreenOnScreen)))
        (Widget|SetVisibility _redscreenfade "Visible")
        (Variables|Default|SetRedScreenOnScreen true)
        (elif (and (not _ishurt) (Variables|Default|GetRedScreenOnScreen))
          (Widget|SetVisibility _redscreenfade "Hidden")
          (Variables|Default|SetRedScreenOnScreen false))))
    (:then_1
      (Transformation|SetWorldRotation (Variables|Character|GetMesh) (Math|Rotator|CombineRotators (Math|Rotator|FindLookatRotation (Math|Vector|MakeVector (.x _returnvalue_2) (.y _returnvalue_2) 0.0) (+ (Math|Vector|MakeVector (.x _returnvalue_3) (.y _returnvalue_3) 0.0) (Math|Vector|MakeVector (.x _returnvalue) (.y _returnvalue) 0.0))) (Math|Rotator|MakeRotator 0.0 0.0 -9e+01)) false false))))

(event EventDash
  (params (Target :type Vector :default "0, 0, 0"))
  ;[1 1 1] Dash
  (if (>= (Variables|Default|GetDashCooldownTime) (Variables|Default|GetDashCooldown))
    (Utilities|FlowControl|DoOnce false :!label _label
      (:Completed
        (Variables|Default|SetIsDodging true)
        (Variables|Default|SetDashCooldownTime 0.0)
        (Collision|SetCollisionResponsetoChannel (Variables|Default|GetCapsuleComponent) "ECC_Pawn" "ECR_Ignore")
        (Character|LaunchCharacter "0.000000,0.000000,200.000000" false false)
        (Utilities|FlowControl|Delay 0.1)
        (Character|LaunchCharacter (* (Math|Vector|GetUnitDirection(Vector) (Transformation|GetActorLocation) Target) (Variables|Default|GetDashForce)) false false)
        (Utilities|FlowControl|Delay 0.4)
        (Collision|SetCollisionResponsetoChannel (Variables|Default|GetCapsuleComponent) "ECC_Pawn" "ECR_Block")
        (Variables|Default|SetIsDodging false)
        (goto _label Reset)))))

(fn ConstructionScript)

(fn PantUIUpdate
  (Variables|/Script/UMG.TextBlock|SetText (Variables|/Game/UI/WBP_Pant.WBP_Pant_C|GetPantText (Variables|Default|GetPantUI)) (Utilities|Text|ToText(Integer) (Variables|/Script/SkellHell.PantCollector|GetPantCollectedAmount (Variables|Default|GetPantCollector)))))

(fn WeaponCooldownUIUpdate
  (Default|SetFillPercentage (Variables|Default|GetWeaponCooldownUI) (Math|Float|Clamp(Float) (/ (Variables|Default|GetCooldownTime) (Variables|Default|GetWeaponCooldown)))))

(fn DashCooldownUIUpdate
  (Default|SetFillPercentage (Variables|Default|GetDashCooldownUI) (Math|Float|Clamp(Float) (/ (Variables|Default|GetDashCooldownTime) (Variables|Default|GetDashCooldown)))))

(fn IsInvincible
  (bind _returnvalue (Class|Health|GetIsInvincible (Variables|Default|GetHealth)))
  (return (or _returnvalue (Variables|Default|GetIsDodging))))