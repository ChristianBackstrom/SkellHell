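; BP_Pantomat is an interactable pants drop-off that banks the player's collected pants as score and wins the game.
; Every tick it compares player distance to its Sphere radius scaled by actor X scale instead of using overlap events, leaving its own Z out of the distance inputs.
; In range, it moves BP_Bones' PantCollector count into the BP_SkellhellGameInstance score, zeroes the count and opens LVL_GameWon.
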(event EventBeginPlay
  (Variables|Default|SetPlayer (Game|Player|GetPlayerPawn 0)))

(event Collision|EventActorBeginOverlap
  (params (OtherActor :type Actor%20Object%20Reference)))

(event EventTick
  (params (DeltaSeconds :type Float%20%28single-precision%29))
  (bind _returnvalue (Transformation|GetActorLocation))
  (bind _player (Variables|Default|GetPlayer))
  (bind _returnvalue_2 (Transformation|GetActorLocation _player))
  (if (< (Math|Vector|Distance(Vector) (Math|Vector|MakeVector (.x _returnvalue_2) (.y _returnvalue_2) (.z _returnvalue_2)) (Math|Vector|MakeVector (.x _returnvalue) (.y _returnvalue) 0.0)) (* (Variables|/Script/Engine.SphereComponent|GetSphereRadius (Variables|Default|GetSphere)) (.x (Transformation|GetActorScale3D))))
    (bind _asbp_bones (Utilities|Casting|CastToBP_Bones (Variables|Default|GetPlayer)))
    (bind _asbp_skellhell_game_instance (Utilities|Casting|CastToBP_SkellhellGameInstance (Game|GetGameInstance)))
    (Default|AddScore _asbp_skellhell_game_instance (Variables|/Script/SkellHell.PantCollector|GetPantCollectedAmount (Variables|/Game/Blueprint/BP_Bones.BP_Bones_C|GetPantCollector _asbp_bones)))
    (Variables|/Script/SkellHell.PantCollector|SetPantCollectedAmount (Variables|/Game/Blueprint/BP_Bones.BP_Bones_C|GetPantCollector _asbp_bones) 0)
    (Game|OpenLevel(byObjectReference) "/Game/Levels/LVL_GameWon.LVL_GameWon")))

(fn ConstructionScript)