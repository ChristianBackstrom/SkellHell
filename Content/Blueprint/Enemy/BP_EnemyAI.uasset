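; Enemy pawn that chases the player and damages them on proximity.
; BeginPlay sets the seeing-player flag without any sight check and issues a single AI MoveTo targeting the player pawn.
; Every Tick it measures distance to the player and, within a short radius, casts to BP_Bones and calls PlayerHit on its Health unless invincible.
; The enemy has no hit cooldown of its own, relying on the player's invincibility check.
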(event Custom|ChasePlayer
  (if (Variables|Default|GetIsSeeingPlayer)
    (AI|AIMoveTo self "0, 0, 0" (Game|Player|GetPlayerPawn 0) 5.0 false)))

(event EventBeginPlay
  (Variables|Default|SetIsSeeingPlayer true)
  (CallFunction|ChasePlayer))

(event EventTick
  (params (DeltaSeconds :type Float%20%28single-precision%29))
  (bind _returnvalue (Game|Player|GetPlayerPawn 0))
  (if (< (Math|Vector|Distance(Vector) (Transformation|GetActorLocation _returnvalue) (Transformation|GetActorLocation self)) 2.5e+02)
    (bind _asbp_bones (Utilities|Casting|CastToBP_Bones _returnvalue))
    (bind _isinvincible (Default|IsInvincible _asbp_bones))
    (if (not _isinvincible)
      (Class|Health|PlayerHit (Variables|/Game/Blueprint/BP_Bones.BP_Bones_C|GetHealth _asbp_bones)))))

(fn ConstructionScript)