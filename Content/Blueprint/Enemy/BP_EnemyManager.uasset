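; Enemy spawner that fills a box area with BP_EnemyAI actors at startup and keeps adding more during play.
; Tick spawns an enemy whenever a randomized cooldown elapses and the live count is below the cap, and prunes invalid entries from the Enemies array.
; Spawn points are re-rolled until clear of the player, and each enemy faces the player and receives a manager reference.
; EnemyDied removes the given enemy from the array.
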(event EventTick
  (params (DeltaSeconds :type Float%20%28single-precision%29))
  (Utilities|FlowControl|Sequence
    (:then_0
      (bind _output_get (Variables|Default|SetTimeSinceLastSpawn (+ DeltaSeconds (Variables|Default|GetTimeSinceLastSpawn))))
      (if (and (>= _output_get (Variables|Default|GetSpawnCooldown)) (< (Utilities|Array|Length (Variables|Default|GetEnemies)) (Variables|Default|GetMaxEnemyAmount)))
        (CallFunction|SpawnActor)))
    (:then_1
      (for _array_element (Variables|Default|GetEnemies)
        (Utilities|IsValid _array_element
          (:Is%20Not%20Valid
            (Utilities|Array|RemoveItem (Variables|Default|GetEnemies) _array_element)))))))

(event EventBeginPlay
  (for _index (range 0 30)
    (CallFunction|SpawnActor)))

(fn ConstructionScript)

(fn SpawnActor
  (bind _returnvalue (Transformation|GetActorLocation))
  (bind _returnvalue_2 (Game|Player|GetPlayerPawn 0))
  (bind _box (Variables|Default|GetBox))
  (bind _returnvalue_3 (Transformation|GetActorLocation _returnvalue_2))
  (bind _boxextent (Variables|/Script/Engine.BoxComponent|GetBoxExtent _box))
  (bind _returnvalue_4 (Math|Random|RandomPointinBoundingBox _returnvalue (Math|Vector|MakeVector (.x _boxextent) (.y _boxextent) 0.0)))
  (LocalVariables|SetSpawnLocation _returnvalue_4)
  (while (< (Math|Vector|Distance(Vector) (Transformation|GetActorLocation _returnvalue_2) (LocalVariables|GetSpawnLocation)) 1e+03)
    (bind _output_get (LocalVariables|SetSpawnLocation _returnvalue_4)))
  (bind _returnvalue_5 (Game|SpawnActorfromClass "/Game/Blueprint/Enemy/BP_EnemyAI.BP_EnemyAI_C" (Math|Transform|MakeTransform _output_get (Math|Rotator|FindLookatRotation _output_get (Math|Vector|MakeVector (.x _returnvalue_3) (.y _returnvalue_3) 0.0)) "1.000000,1.000000,1.000000") "Undefined" "MultiplyWithRoot" 0 self 0))
  (Utilities|Array|Add (Variables|Default|GetEnemies) _returnvalue_5)
  (Variables|Default|SetSpawnCooldown (Math|Random|RandomFloatinRange (Variables|Default|GetEnemyMinSpawnTime) (Variables|Default|GetEnemyMaxSpawnTime)))
  (Variables|Default|SetTimeSinceLastSpawn 0.0))

(fn EnemyDied
  (params (Enemy :type Actor%20Object%20Reference))
  (bind _asbp_enemy_ai (Utilities|Casting|CastToBP_EnemyAI Enemy))
  (Utilities|Array|RemoveItem (Variables|Default|GetEnemies) _asbp_enemy_ai))