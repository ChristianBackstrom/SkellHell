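; BP_SkellhellGameInstance is the game instance for Skellhell, holding a list of scores, the music component and the music volume.
; AddScore appends to the score list.
; StartMusic creates the Animal track as a 2D sound that persists across level transitions without auto-destroy, reuses it while valid, and plays it only if it is not already playing.
; ChangeVolume applies the stored Volume to the existing music component.
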(fn AddScore
  (params (Score :type Integer))
  (Utilities|Array|Add (Variables|Default|GetScores) Score)
  (return))

(fn StartMusic
  (Utilities|IsValid (Variables|Default|GetMusic)
    (:Is%20Valid
      _)
    (:Is%20Not%20Valid
      (bind _returnvalue (Audio|CreateSound2D "/Game/Sound/Animal.Animal" (Variables|Default|GetVolume) 1.0 0.0 0 true false))
      (Variables|Default|SetMusic _returnvalue)))
  (if (not (Audio|Components|Audio|IsPlaying (Variables|Default|GetMusic)))
    (Audio|Components|Audio|Play (Variables|Default|GetMusic) 0.0)))

(fn ChangeVolume
  (bind _music (Variables|Default|GetMusic))
  (Utilities|IsValid _music
    (:Is%20Valid
      (Audio|Components|Audio|SetVolumeMultiplier _music (Variables|Default|GetVolume) :!class /Script/Engine.AudioComponent))))